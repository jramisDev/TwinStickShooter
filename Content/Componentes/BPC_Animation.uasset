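; Animation component for a Paper2D character, picking a facing direction and idle or moving status from owner velocity every tick.
; Normalized velocity sets one of four directions, which selects the top, bottom or side flipbook map.
; Left and right share the side map, with the sprite rotated to mirror it.
; The flipbook swap is disconnected, so only rotation reaches the lazily cached owner's sprite.
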(event `self.ReceiveTick`
  (params (DeltaSeconds :type "Float (single-precision)"))
  (`self.AnimationStatus`))

(fn `AnimationStatus`
  (locals (MapToUse :type "Map of /Game/Blueprints/Enums/E_AnimationStatus Enum to PaperFlipbook Object Reference") (NewAnimationStatus :type "/Game/Blueprints/Enums/E_AnimationStatus Enum"))
  (bind _sideanimation (`self.SideAnimation`))
  (`self.setDirection`)
  (if (!= (`self.getParentVelocity`) (0.0 0.0 0.0) :`ErrorTolerance` 0.01)
    (set `local.NewAnimationStatus` "NewEnumerator2")
    (else
      (set `local.NewAnimationStatus` "NewEnumerator1")))
  (set `self.StatusAnimation` (`local.NewAnimationStatus`))
  (set `local.MapToUse` (select `/Game/Blueprints/Enums/E_AnimationDirection` (`self.Direction`) :`NewEnumerator0` (`self.TopAnimation`) :`NewEnumerator1` (`self.BotAnimation`) :`NewEnumerator2` _sideanimation :`NewEnumerator3` _sideanimation))
  (`SceneComponent.K2_SetRelativeRotation` (`self.getParentFlipbook`) (`KismetMathLibrary.MakeRotator` 90.0 (select `/Game/Blueprints/Enums/E_AnimationDirection` (`self.Direction`) :`NewEnumerator2` -180.0 :!type "Float (single-precision)") -90.0) false false))

(fn `getDirection`
  (returns (Direction :type "/Game/Blueprints/Enums/E_AnimationDirection Enum"))
  (return (`self.Direction`)))

(fn `getOwnerReference`
  (returns (Owner :type "PaperCharacter Object Reference"))
  (`self.Owner`
    (:`then`
      _)
    (:`else`
      (bind _aspaper_character (cast `PaperCharacter` (`self.GetOwner`)))
      (bind _output_get (set `self.Owner` _aspaper_character))))
  (return _output_get))

(fn `getParentFlipbook`
  (returns (`Paper Flipbook Component` :type "PaperFlipbookComponent Object Reference"))
  (return (`PaperCharacter.Sprite` (`self.getOwnerReference`))))

(fn `getParentVelocity`
  (returns (Velocity :type "Vector Structure"))
  (return (`MovementComponent.Velocity` (`Character.CharacterMovement` (`self.getOwnerReference`)))))

(fn `setAnimation`
  (params (StatusAnimation :type "/Game/Blueprints/Enums/E_AnimationStatus Enum" :default "NewEnumerator0"))
  (set `self.StatusAnimation` StatusAnimation))

(fn `setDirection`
  (bind _returnvalue (`KismetMathLibrary.Conv_VectorToVector2D` (`self.getParentVelocity`)))
  (bind (_x _y) (`KismetMathLibrary.BreakVector2D` (`KismetMathLibrary.Normal2D` _returnvalue)))
  (if (!= _returnvalue (0.0 0.0) :`ErrorTolerance` 0.1)
    (if (> _x 0.5)
      (set `self.Direction` "NewEnumerator0")
      (elif (< _x -0.5)
        (set `self.Direction` "NewEnumerator1")
        (elif (> _y 0.0)
          (set `self.Direction` "NewEnumerator2")
          (else
            (set `self.Direction` "NewEnumerator3")))))))