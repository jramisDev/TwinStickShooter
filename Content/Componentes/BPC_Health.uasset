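; BPC_Health is a health component that tracks and clamps an actor's health as it takes damage.
; On BeginPlay it fills health to maximum, first scaling that maximum by the GameInstance difficulty multiplier for BP_EnemyBase owners.
; SufferDamage destroys the owner at zero health, except Hero2D, which only prints a death message because the Game Over level load is disconnected.
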(event `self.ReceiveBeginPlay`
  (`self.init`))

(fn `Die`
  (`Actor.K2_DestroyActor` (`self.GetOwner`)))

(fn `getHealth`
  (returns (Health :type "Float (double-precision)"))
  (return (`self.Health`)))

(fn `getHero2D`
  (returns (Hero2D :type "/Game/Blueprints/Player/Hero2D Object Reference"))
  (`self.Hero2D`
    (:`then`
      _)
    (:`else`
      (bind _ashero_2d (cast `/Game/Blueprints/Player/Hero2D` (`GameplayStatics.GetPlayerPawn` 0)))
      (set `self.Hero2D` _ashero_2d)))
  (return (`self.Hero2D`)))

(fn `init`
  (cast `/Game/Blueprints/Base/BP_EnemyBase` (`self.GetOwner`)
    (:`then`
      (bind _output_get (set `self.HealthMax` (* (`/Game/Blueprints/Comunes/GI_Game.MultiplierDifficulty` (`/Game/Blueprints/FunctionsLibrary/BFL_General.getGIReference`)) (`self.HealthMax`))))
      (set `self.Health` _output_get))
    (:`CastFailed`
      (set `self.Health` (`self.HealthMax`)))))

(fn `SufferDamage`
  (params (Damage :type "Float (double-precision)") (DamageType :type "DamageType Object Reference"))
  (bind _returnvalue (`self.GetOwner`))
  (bind _output_get (set `self.Health` (`KismetMathLibrary.FClamp` (- (`self.Health`) Damage) 0.0 (`self.HealthMax`))))
  (if (<= _output_get 0.0)
    (cast `/Game/Blueprints/Player/Hero2D` _returnvalue
      (:`then`
        (`KismetSystemLibrary.PrintString` "HAS MUERTO!" true true (struct :`R` 1.0 :`A` 1.0)))
      (:`CastFailed`
        (`Actor.K2_DestroyActor` _returnvalue)))))