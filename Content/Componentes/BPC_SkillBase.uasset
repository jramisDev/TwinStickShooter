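; Base skill component for paper characters that fires projectiles, gated by a cooldown and the owner's animation state.
; CastSkill starts a cast-time timer and spawns the Projectile class facing the given direction.
; ReduceCastTime decrements cast time, restoring walking movement and changing animation when it runs out.
; The AttackSpeed cooldown timer starts only on a rejected cast attempt, not on firing, and re-enables firing when done.
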(event `ReduceCastTime`
  (params (CastTimeTimer :type "TimerHandle Structure"))
  (set `self.CastTimeTimer` CastTimeTimer))

(event `CastSkill`
  (params (Origen :type "Vector Structure") (Direction :type "Vector Structure") (projectile :type "/Game/Blueprints/Base/BP_BaseProjectile Class Reference"))
  (if (and (`self.CanIFire`) (not (`KismetArrayLibrary.Array_Contains` (`|MakeArray` "NewEnumerator4" "NewEnumerator6" "NewEnumerator7" :!type "/Game/Blueprints/Enums/E_AnimationStatus Enum") (`/Game/Componentes/BPC_Animation.StatusAnimation` (`self.GetOwnerStatusMachine`)))))
    (set `self.CanIFire` false)
    (`self.StartCastTime`)
    (`self.SpawnProjectiles` Origen (+ Origen (* Direction 500.0)))
    (elif (not (`KismetSystemLibrary.K2_IsTimerActiveHandle` (`self.Timer Coldwon`)))
      (bind _returnvalue (`KismetSystemLibrary.K2_SetTimerDelegate` (delegate `RestartColdDown`) (`self.Attack Speed`)))
      (set `self.Timer Coldwon` _returnvalue))))

(event `RestartColdDown`
  (set `self.CanIFire` true)
  (`KismetSystemLibrary.K2_ClearAndInvalidateTimerHandle` (`self.Timer Coldwon`)))

(event `SpawnProjectiles`
  (params (Origen :type "Vector Structure") (Direccion :type "Vector Structure"))
  (bind (_x _y _z) (`KismetMathLibrary.BreakVector3f` Origen))
  (`|SpawnActorFromClass` (`self.Projectile`) (`KismetMathLibrary.MakeTransform` (`KismetMathLibrary.MakeVector` _x _y (- _z 10.0)) (`KismetMathLibrary.FindLookAtRotation` Origen Direccion)) "Undefined" "OverrideRootScale" (`self.Get Owner Ref`) 3 (cast `/Game/Blueprints/Base/BP_EnemyBase` (`self.GetOwner`) :!pure true)))

(fn `Get Owner Ref`
  (returns (`As PaperCharacterBase` :type "/Game/Blueprints/Base/BP_PaperCharacterBase Object Reference"))
  (`self.As PaperCharacterBase`
    (:`then`
      _)
    (:`else`
      (bind _asbp_paper_character_base (cast `/Game/Blueprints/Base/BP_PaperCharacterBase` (`self.GetOwner`)))
      (set `self.As PaperCharacterBase` _asbp_paper_character_base)))
  (return (`self.As PaperCharacterBase`)))

(fn `GetOwnerMovementComponent`
  (returns (`Character Movement` :type "CharacterMovementComponent Object Reference"))
  (return (`Character.CharacterMovement` (`self.Get Owner Ref`))))

(fn `GetOwnerStatusMachine`
  (returns (BPA_Animation :type "/Game/Componentes/BPC_Animation Object Reference"))
  (return (`/Game/Blueprints/Base/BP_PaperCharacterBase.BPC_Animation` (`self.Get Owner Ref`))))

(fn `Reduce Cast Time`
  (bind _output_get (set `self.CastTime` (- (`self.CastTime`) (`self.CastTimeTickTime`))))
  (if (<= _output_get 0.0)
    (`KismetSystemLibrary.K2_ClearAndInvalidateTimerHandle` (`self.CastTimeTimer`))
    (`CharacterMovementComponent.SetMovementMode` (`self.GetOwnerMovementComponent`) "MOVE_Walking" 0)
    (`/Game/Componentes/BPC_Animation.setAnimation` (`self.GetOwnerStatusMachine`) "NewEnumerator1")))

(fn `StartCastTime`
  (if (> (`self.CastTimeMax`) 0.0)
    (set `self.CastTime` (`self.CastTimeMax`))
    (bind _returnvalue (`KismetSystemLibrary.K2_SetTimerDelegate` (`|CreateDelegate` :!event `Reduce Cast Time`) (`self.CastTimeTickTime`)))
    (set `self.CastTimeTimer` _returnvalue)))