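; Skill component that fires a cone-shaped spread of projectiles from an origin point, assigned to its owner.
; SpawnProjectiles aims the first shot with a look-at rotation toward Direccion, treated as a target point.
; Later shots alternate either side in yaw, stepping outward by MaxAngle divided by ProjectileNumber minus one.
; Odd counts give a symmetric cone; a single projectile makes that divisor zero.
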(event `self.SpawnProjectiles`
  (params (Origen :type "Vector Structure") (Direccion :type "Vector Structure"))
  (bind (_returnvalue_roll _returnvalue_pitch _returnvalue_yaw) (`KismetMathLibrary.BreakRotator` (`KismetMathLibrary.FindLookAtRotation` Origen Direccion)))
  (set `self.IncreaseAngle` 0)
  (for _index (range (`self.ProjectileNumber`))
    (bind _returnvalue (== (mod _index 2) 0))
    (`|SpawnActorFromClass` (`self.Projectile`) (`KismetMathLibrary.MakeTransform` Origen (`KismetMathLibrary.MakeRotator` _returnvalue_roll _returnvalue_pitch (+ _returnvalue_yaw (* (/ (`self.MaxAngle`) (- (`self.ProjectileNumber`) 1)) (`self.IncreaseAngle`) (select `bool` _returnvalue :`false` -1.0 :`true` 1.0))))) "Undefined" "OverrideRootScale" (`self.Get Owner Ref`) 3 null)
    (if _returnvalue
      (`/Engine/EditorBlueprintResources/StandardMacros.IncrementInt` (`self.IncreaseAngle`)))))