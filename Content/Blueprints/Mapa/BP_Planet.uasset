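; BP_Planet is a level-select planet on the map, driven by a Planet data struct.
; On BeginPlay it loads the planet's sprite, darkens it if unvisited, and shows a text label only if the level is beaten.
; OpenLevel marks the matching entry in the GameInstance's LevelData array as visited, then opens that level by name.
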(event `self.ReceiveBeginPlay`
  (bind (_planet_level_name _planet_sprite _planet_visitado _planet_superado) (break `/Game/Structs/S_LevelData` (`self.Planet`)))
  (bind _returnvalue (`KismetSystemLibrary.LoadAsset_Blocking` _planet_sprite))
  (bind _aspaper_sprite (cast `PaperSprite` _returnvalue))
  (`PaperSpriteComponent.SetSprite` (`self.PaperSprite`) _aspaper_sprite)
  (`PaperSpriteComponent.SetSpriteColor` (`self.PaperSprite`) (select `bool` _planet_visitado :`false` (struct :`R` 0.161458 :`G` 0.161458 :`B` 0.161458 :`A` 1.0) :`true` (struct :`R` 1.0 :`G` 1.0 :`B` 1.0 :`A` 1.0) :!type "LinearColor Structure"))
  (`SceneComponent.SetHiddenInGame` (`self.TextRender`) (select `bool` _planet_superado :`false` true) false))

(event `OpenLevel`
  (bind _planet_level_name (break `/Game/Structs/S_LevelData` (`self.Planet`)))
  (for (_array_element _array_index) (`/Game/Blueprints/Comunes/GI_Game.LevelData` (`/Game/Blueprints/FunctionsLibrary/BFL_General.getGIReference`))
    (if (== (break `/Game/Structs/S_LevelData` _array_element) _planet_level_name)
      (`KismetArrayLibrary.Array_Set` (`/Game/Blueprints/Comunes/GI_Game.LevelData` (`/Game/Blueprints/FunctionsLibrary/BFL_General.getGIReference`)) _array_index (make `/Game/Structs/S_LevelData` (break `/Game/Structs/S_LevelData` _array_element) (`.SPRITE_28_CD2009C2430A6C0C6A2092A1CE780978` (break `/Game/Structs/S_LevelData` _array_element)) true (`.SUPERADO_9_B1F6AB9C469581F20DA140BA1916F819` (break `/Game/Structs/S_LevelData` _array_element)) (`.NEXT_LEVEL_31_B4A7B5754A2EA9B6E7CB6385A0F8C050` (break `/Game/Structs/S_LevelData` _array_element))))
      (break)))
  (`GameplayStatics.OpenLevel` _planet_level_name))

(fn `UserConstructionScript`)