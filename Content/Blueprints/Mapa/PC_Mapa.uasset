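; Player controller for the map, where the player moves a pawn and clicks planets to open levels.
; On possession it caches the PAWN_Mapa, shows the cursor and focuses the game viewport; BeginPlay adds the IMC_Mapa Enhanced Input context.
; Movement input calls the pawn's MovementInput.
; Left click, on both Started and Triggered, prints debug text, traces under the cursor and calls OpenLevelByName on any BP_Planet hit.
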(event `self.ReceivePossess`
  (params (PossessedPawn :type "Pawn Object Reference"))
  ;[1 1 1] Poseemos el pawn
  (bind _aspawn_mapa (cast `/Game/Blueprints/Mapa/PAWN_Mapa` PossessedPawn))
  (set `self.As Pawn` _aspawn_mapa)
  (set `self.bShowMouseCursor` true)
  (`WidgetBlueprintLibrary.SetFocusToGameViewport`))

(event `self.ReceiveBeginPlay`
  ;[1 1 1] Inputs generales del juego
  (`EnhancedInputSubsystemInterface.AddMappingContext` (subsystem `EnhancedInputLocalPlayerSubsystem`) "/Game/Inputs/IMC_Mapa.IMC_Mapa" 0 (struct)))

(event `EnhancedInput|/Game/Inputs/IA_Movement`
  (params (ActionValue :type "Vector2D Structure") (ElapsedSeconds :type "Float (double-precision)") (TriggeredSeconds :type "Float (double-precision)") (InputAction :type "InputAction Object Reference" :default "/Game/Inputs/IA_Movement.IA_Movement"))
  (:`Triggered`
    (`/Game/Blueprints/Mapa/PAWN_Mapa.MovementInput` (`self.As Pawn`))))

(event `EnhancedInput|/Game/Inputs/IA_LeftButtonMouse`
  (params (ActionValue :type Boolean) (ElapsedSeconds :type "Float (double-precision)") (TriggeredSeconds :type "Float (double-precision)") (InputAction :type "InputAction Object Reference" :default "/Game/Inputs/IA_LeftButtonMouse.IA_LeftButtonMouse"))
  (bind (_hitresult _returnvalue) (`self.GetHitResultUnderCursorByChannel` "TraceTypeQuery1"))
  (:`Triggered`
    (`KismetSystemLibrary.PrintString` "Hello")
    (if _returnvalue :!label _label
      (bind _asbp_planet (cast `/Game/Blueprints/Mapa/BP_Planet` (`.HitActor` (`GameplayStatics.BreakHitResult` _hitresult))))
      (`/Game/Blueprints/Mapa/BP_Planet.OpenLevel` _asbp_planet)))
  (:`Started`
    (`KismetSystemLibrary.PrintString` "Hello")
    (goto _label)))

(fn `UserConstructionScript`)