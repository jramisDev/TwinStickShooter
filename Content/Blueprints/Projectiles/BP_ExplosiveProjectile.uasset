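; Timed explosive projectile that stops one second before its lifespan ends and detonates, playing a Paper2D impact flipbook before destroying itself.
; On detonation, the sphere switches to the PlayerShoot or EnemyShoot collision profile, depending on whether its owner is the player's pawn.
; The sphere's begin-overlap event applies base damage to whatever it touches.
; Detonation is purely timer-driven; overlaps never trigger it.
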(event `self.ReceiveBeginPlay`
  (bind _scaleprojectile (`self.ScaleProjectile`))
  (bind _lifespan (`self.LifeSpan`))
  (`parent.ReceiveBeginPlay`)
  (`self.SetActorScale3D` (`KismetMathLibrary.MakeVector` _scaleprojectile _scaleprojectile _scaleprojectile))
  (`self.SetLifeSpan` _lifespan)
  (`KismetSystemLibrary.K2_SetTimerDelegate` (delegate `Activate`) (- _lifespan 1.0)))

(event `Activate`
  (bind _paperflipbook (`self.PaperFlipbook`))
  (`MovementComponent.StopMovementImmediately` (`self.ProjectileMovement`))
  (`PrimitiveComponent.SetCollisionProfileName` (`self.Sphere`) (select `bool` (== (`Controller.K2_GetPawn` (`GameplayStatics.GetPlayerController` 0)) (`self.GetOwner`)) :`false` "EnemyShoot" :`true` "PlayerShoot" :!type "Name") true)
  (`PaperFlipbookComponent.SetFlipbook` _paperflipbook (`self.EfectoColision`))
  (`PaperFlipbookComponent.PlayFromStart` _paperflipbook)
  (`KismetSystemLibrary.Delay` (`PaperFlipbookComponent.GetFlipbookLength` _paperflipbook))
  (`self.K2_DestroyActor`))

(event `self.Sphere.OnComponentBeginOverlap`
  (params (OverlappedComponent :type "PrimitiveComponent Object Reference") (OtherActor :type "Actor Object Reference") (OtherComp :type "PrimitiveComponent Object Reference") (OtherBodyIndex :type Integer) (bFromSweep :type Boolean) (SweepResult :type "HitResult Structure (by ref)"))
  (`GameplayStatics.ApplyDamage` OtherActor (`self.DamageBase`)))

(fn `UserConstructionScript`)