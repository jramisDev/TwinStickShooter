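; BP_ShotProjectile is a 2D flipbook projectile that damages actors it overlaps and can pierce several before expiring.
; BeginPlay sets scale and lifespan, then picks a PlayerShoot or EnemyShoot capsule collision profile depending on whether the owner is the player's pawn.
; Overlap applies damage and plays the impact flipbook, then decrements Pierce after that animation's length, destroying itself at zero.
; Ending an overlap restores the normal flipbook.
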(event `self.ReceiveBeginPlay`
  (bind _scaleprojectile (`self.ScaleProjectile`))
  (`parent.ReceiveBeginPlay`)
  (`self.SetActorScale3D` (`KismetMathLibrary.MakeVector` _scaleprojectile _scaleprojectile _scaleprojectile))
  (`self.SetLifeSpan` (`self.LifeSpan`))
  (`PrimitiveComponent.SetCollisionProfileName` (`self.Capsule`) (select `bool` (== (`Controller.K2_GetPawn` (`GameplayStatics.GetPlayerController` 0)) (`self.GetOwner`)) :`false` "EnemyShoot" :`true` "PlayerShoot" :!type "Name") true))

(event `self.Capsule.OnComponentBeginOverlap`
  (params (OverlappedComponent :type "PrimitiveComponent Object Reference") (OtherActor :type "Actor Object Reference") (OtherComp :type "PrimitiveComponent Object Reference") (OtherBodyIndex :type Integer) (bFromSweep :type Boolean) (SweepResult :type "HitResult Structure (by ref)"))
  (bind _paperflipbook (`self.PaperFlipbook`))
  (`GameplayStatics.ApplyDamage` OtherActor (`self.Damage`))
  (`PaperFlipbookComponent.SetFlipbook` _paperflipbook (`self.EfectoColision`))
  (`PaperFlipbookComponent.PlayFromStart` _paperflipbook)
  (`KismetSystemLibrary.Delay` (`PaperFlipbookComponent.GetFlipbookLength` _paperflipbook))
  (bind _result (`/Engine/EditorBlueprintResources/StandardMacros.DecrementInt` (`self.Pierce`))
    (:`  `
      (if (<= _result 0)
        (`self.K2_DestroyActor`)))))

(event `self.Capsule.OnComponentEndOverlap`
  (params (OverlappedComponent :type "PrimitiveComponent Object Reference") (OtherActor :type "Actor Object Reference") (OtherComp :type "PrimitiveComponent Object Reference") (OtherBodyIndex :type Integer))
  (`PaperFlipbookComponent.SetFlipbook` (`self.PaperFlipbook`) (`self.EfectoNormal`)))

(fn `UserConstructionScript`)