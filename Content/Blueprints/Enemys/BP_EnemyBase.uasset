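; BP_EnemyBase is a base enemy Blueprint that attacks the player and deals contact damage.
; Its ShootToPlayer event casts a skill through BPCSkillBase from the enemy's location, passing the X and Y direction toward the player's pawn.
; Overlapping the capsule applies a small fixed damage to any Hero2D.
; The file shows nothing that triggers the shot itself.
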(event `ShootToPlayer`
  (bind _returnvalue (`self.K2_GetActorLocation`))
  (bind (_returnvalue_x _returnvalue_y) (`KismetMathLibrary.BreakVector` (`KismetMathLibrary.GetForwardVector` (`KismetMathLibrary.FindLookAtRotation` _returnvalue (`self.K2_GetActorLocation` (`Controller.K2_GetPawn` (`GameplayStatics.GetPlayerController` 0)))))))
  (`/Game/Componentes/BPC_SkillBase.CastSkill` (`self.BPC_SkillBase`) _returnvalue (`KismetMathLibrary.MakeVector` _returnvalue_x _returnvalue_y)))

(event `self.CapsuleComponent.OnComponentBeginOverlap`
  (params (OverlappedComponent :type "PrimitiveComponent Object Reference") (OtherActor :type "Actor Object Reference") (OtherComp :type "PrimitiveComponent Object Reference") (OtherBodyIndex :type Integer) (bFromSweep :type Boolean) (SweepResult :type "HitResult Structure (by ref)"))
  (bind _ashero_2d (cast `/Game/Blueprints/Player/Hero2D` OtherActor))
  (`GameplayStatics.ApplyDamage` _ashero_2d 5.0))

(fn `UserConstructionScript`)