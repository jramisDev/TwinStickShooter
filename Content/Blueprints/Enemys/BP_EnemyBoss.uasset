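; Boss enemy Blueprint that tracks which of three combat phases it is in, based on remaining health.
; It starts in the first phase, then every Tick converts health from its BPCHealth component into a percentage and sets BossMode against two descending thresholds.
; This file only sets the phase and defines no behavior for each one.
; Logic to yaw the sprite toward its target is present but disconnected.
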(event EventBeginPlay
  (Variables|Default|SetBossMode "NewEnumerator0"))

(event EventTick
  (params (DeltaSeconds :type Float%20%28single-precision%29))
  (CallFunction|ChangeFaseStatus))

(fn ConstructionScript
  (|CallParentFunction))

(fn ChangeFaseStatus
  (bind _bpc_health (Variables|Default|GetBPC_Health))
  (bind _health (Default|GetHealth _bpc_health))
  (bind _healthmax (Variables|/Game/Componentes/BPC_Health.BPC_Health_C|GetHealthMax _bpc_health))
  (bind _returnvalue (|((Health*100)/HealtMax) _health _healthmax))
  (if (>= _returnvalue 75.0)
    (Variables|Default|SetBossMode "NewEnumerator0")
    (elif (>= _returnvalue 4e+01)
      (Variables|Default|SetBossMode "NewEnumerator1")
      (else
        (Variables|Default|SetBossMode "NewEnumerator2")))))