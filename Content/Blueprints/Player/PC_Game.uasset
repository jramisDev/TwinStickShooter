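; Player controller for the game that routes Enhanced Input to the possessed Hero2D pawn.
; On possession it caches the pawn as Hero2D, and on BeginPlay it adds the IMC_Game mapping context and focuses the game viewport.
; Movement, aim, shoot, weapon selection, dash and escape actions each forward directly to a matching input function on the hero, keeping gameplay logic out of the controller.
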(event `self.ReceivePossess`
  (params (PossessedPawn :type "Pawn Object Reference"))
  ;[1 1 1] Poseemos el pawn
  (bind _ashero_2d (cast `/Game/Blueprints/Player/Hero2D` PossessedPawn))
  (set `self.As Hero2D` _ashero_2d))

(event `self.ReceiveBeginPlay`
  ;[1 1 1] Inputs generales del juego
  (`EnhancedInputSubsystemInterface.AddMappingContext` (subsystem `EnhancedInputLocalPlayerSubsystem`) "/Game/Inputs/IMC_Game.IMC_Game" 0 (struct))
  ;[1 1 1] Nos ahorramos el click a la hora de entrar
  (`WidgetBlueprintLibrary.SetFocusToGameViewport`))

(event `EnhancedInput|/Game/Inputs/IA_Movement`
  (params (ActionValue :type "Vector2D Structure") (ElapsedSeconds :type "Float (double-precision)") (TriggeredSeconds :type "Float (double-precision)") (InputAction :type "InputAction Object Reference" :default "/Game/Inputs/IA_Movement.IA_Movement"))
  (:`Triggered`
    (`/Game/Blueprints/Player/Hero2D.InputMovement` (`self.As Hero2D`) ActionValue)))

(event `EnhancedInput|/Game/Inputs/IA_Aim`
  (params (ActionValue :type "Float (double-precision)") (ElapsedSeconds :type "Float (double-precision)") (TriggeredSeconds :type "Float (double-precision)") (InputAction :type "InputAction Object Reference" :default "/Game/Inputs/IA_Aim.IA_Aim"))
  (:`Triggered`
    (`/Game/Blueprints/Player/Hero2D.InputAim` (`self.As Hero2D`) ActionValue)))

(event `EnhancedInput|/Game/Inputs/IA_Shoot`
  (params (ActionValue :type Boolean) (ElapsedSeconds :type "Float (double-precision)") (TriggeredSeconds :type "Float (double-precision)") (InputAction :type "InputAction Object Reference" :default "/Game/Inputs/IA_Shoot.IA_Shoot"))
  (:`Started`
    (`/Game/Blueprints/Player/Hero2D.InputShoot` (`self.As Hero2D`))))

(event `EnhancedInput|/Game/Inputs/IA_PrimaryWeapon`
  (params (ActionValue :type Boolean) (ElapsedSeconds :type "Float (double-precision)") (TriggeredSeconds :type "Float (double-precision)") (InputAction :type "InputAction Object Reference" :default "/Game/Inputs/IA_PrimaryWeapon.IA_PrimaryWeapon"))
  (:`Started`
    (`/Game/Blueprints/Player/Hero2D.InputPrimaryWeapon` (`self.As Hero2D`))))

(event `EnhancedInput|/Game/Inputs/IA_SecondaryWeapon`
  (params (ActionValue :type Boolean) (ElapsedSeconds :type "Float (double-precision)") (TriggeredSeconds :type "Float (double-precision)") (InputAction :type "InputAction Object Reference" :default "/Game/Inputs/IA_SecondaryWeapon.IA_SecondaryWeapon"))
  (:`Started`
    (`/Game/Blueprints/Player/Hero2D.InputSecondaryWeapon` (`self.As Hero2D`))))

(event `EnhancedInput|/Game/Inputs/IA_TertiaryWeapon`
  (params (ActionValue :type Boolean) (ElapsedSeconds :type "Float (double-precision)") (TriggeredSeconds :type "Float (double-precision)") (InputAction :type "InputAction Object Reference" :default "/Game/Inputs/IA_TertiaryWeapon.IA_TertiaryWeapon"))
  (:`Started`
    (`/Game/Blueprints/Player/Hero2D.InputTertiaryWeapon` (`self.As Hero2D`))))

(event `EnhancedInput|/Game/Inputs/IA_Dash`
  (params (ActionValue :type Boolean) (ElapsedSeconds :type "Float (double-precision)") (TriggeredSeconds :type "Float (double-precision)") (InputAction :type "InputAction Object Reference" :default "/Game/Inputs/IA_Dash.IA_Dash"))
  (:`Started`
    (`/Game/Blueprints/Player/Hero2D.InputDash` (`self.As Hero2D`))))

(event `EnhancedInput|/Game/Inputs/IA_Escape`
  (params (ActionValue :type Boolean) (ElapsedSeconds :type "Float (double-precision)") (TriggeredSeconds :type "Float (double-precision)") (InputAction :type "InputAction Object Reference" :default "/Game/Inputs/IA_Escape.IA_Escape"))
  (:`Started`
    (`/Game/Blueprints/Player/Hero2D.InputEscape` (`self.As Hero2D`) true)))

(fn `UserConstructionScript`)