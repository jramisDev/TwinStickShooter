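; Player hero Blueprint that handles input for movement, aiming, shooting, weapon selection, dashing and pausing.
; Movement feeds the 2D input into CharacterMovement and stores the last non-zero direction.
; Shoot, weapon and dash inputs are print-string placeholders, and aim only prints and zeroes the actor rotation.
; Escape pauses the game and opens the pause menu through a lazily cached HUD_Game reference.
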(event `InputMovement`
  (params (`Action Value` :type "Vector2D Structure"))
  (bind _returnvalue (`KismetMathLibrary.Conv_Vector2DToVector` `Action Value`))
  (`PawnMovementComponent.AddInputVector` (`self.CharacterMovement`) _returnvalue false)
  (if (!= _returnvalue (0.0 0.0 0.0) :`ErrorTolerance` 0.1)
    (set `self.LastDirection` _returnvalue)))

(event `InputAim`
  (params (`Action Value` :type "Float (double-precision)"))
  (`KismetSystemLibrary.PrintString` "Hello")
  (`self.K2_SetActorRotation` (struct) true))

(event `InputShoot`
  (`KismetSystemLibrary.PrintString` "Shoot"))

(event `InputPrimaryWeapon`
  (`KismetSystemLibrary.PrintString` "Primary Weapon"))

(event `InputSecondaryWeapon`
  (`KismetSystemLibrary.PrintString` "Secondary Weapon"))

(event `InputTertiaryWeapon`
  (`KismetSystemLibrary.PrintString` "Tertiary Weapon"))

(event `InputDash`
  (`KismetSystemLibrary.PrintString` "Dash"))

(event `InputEscape`
  (`GameplayStatics.SetGamePaused` true)
  (`/Game/Levels/LevelsGame/HUD_Game.OpenPauseMenu` (`self.getHUDRef`)))

(fn `getHUDRef`
  (returns (HUD_Game :type "/Game/Levels/LevelsGame/HUD_Game Object Reference"))
  (`self.As HUD_Game`
    (:`then`
      _)
    (:`else`
      (bind _ashud_game (cast `/Game/Levels/LevelsGame/HUD_Game` (`PlayerController.GetHUD` (`GameplayStatics.GetPlayerController` 0))))
      (set `self.As HUD_Game` _ashud_game)))
  (return (`self.As HUD_Game`)))

(fn `UserConstructionScript`)