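; Base projectile Blueprint that damages actors its capsule overlaps.
; On BeginPlay it applies its scale and lifespan, then picks the PlayerShoot or EnemyShoot collision profile based on whether its owner is the first player's controlled pawn.
; Each overlap applies damage and decrements a pierce count, destroying the projectile once that count is used up.
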(event `self.ReceiveBeginPlay`
  (bind _scaleprojectile (`self.ScaleProjectile`))
  (bind _returnvalue (== (`Controller.K2_GetPawn` (`GameplayStatics.GetPlayerController` 0)) (`self.GetOwner`)))
  (`self.SetActorScale3D` (`KismetMathLibrary.MakeVector` _scaleprojectile _scaleprojectile _scaleprojectile))
  (`self.SetLifeSpan` (`self.LifeSpan`))
  (`PrimitiveComponent.SetCollisionProfileName` (`self.Capsule`) (select `bool` _returnvalue :`false` "EnemyShoot" :`true` "PlayerShoot" :!type "Name") true)
  (if _returnvalue
    _))

(event `self.Capsule.OnComponentBeginOverlap`
  (params (OverlappedComponent :type "PrimitiveComponent Object Reference") (OtherActor :type "Actor Object Reference") (OtherComp :type "PrimitiveComponent Object Reference") (OtherBodyIndex :type Integer) (bFromSweep :type Boolean) (SweepResult :type "HitResult Structure (by ref)"))
  (`GameplayStatics.ApplyDamage` OtherActor (`self.Damage`))
  (bind _result (`/Engine/EditorBlueprintResources/StandardMacros.DecrementInt` (`self.Pierce`))
    (:`  `
      (if (<= _result 0)
        (`self.K2_DestroyActor`)))))

(fn `UserConstructionScript`)