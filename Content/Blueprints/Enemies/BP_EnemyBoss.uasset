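; Boss enemy Blueprint that starts in its first phase, turns toward the pawn and prints its health on screen every tick.
; ChangeFaseStatus picks one of three boss modes from the health component's remaining percentage.
; GoToNextLevel finds the current level in the GameInstance level data and opens its configured next level.
; Neither function is called within this Blueprint's own graphs.
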(event EventBeginPlay
  (|CallParentFunction)
  (Variables|Default|SetBossMode "NewEnumerator0"))

(event EventTick
  (params (DeltaSeconds :type Float%20%28single-precision%29))
  (bind _bpc_health (Variables|Default|GetBPC_Health))
  (Development|PrintText (Utilities|Text|FormatText "Health: {h} / HealthMax: {hm}" (Default|GetHealth _bpc_health) (Variables|/Game/Componentes/BPC_Health.BPC_Health_C|GetHealthMax _bpc_health)) true true "(R=0.000000,G=0.660000,B=1.000000,A=1.000000)" 0.05)
  (CallFunction|SetRotationtoPawn))

(fn ConstructionScript
  (|CallParentFunction))

(fn ChangeFaseStatus
  (bind _bpc_health (Variables|Default|GetBPC_Health))
  (bind _health (Default|GetHealth _bpc_health))
  (bind _healthmax (Variables|/Game/Componentes/BPC_Health.BPC_Health_C|GetHealthMax _bpc_health))
  (bind _returnvalue (|((Health*100)/HealtMax) _health _healthmax))
  (if (>= _returnvalue 75.0)
    (Variables|Default|SetBossMode "NewEnumerator0")
    (elif (>= _returnvalue 4e+01)
      (Variables|Default|SetBossMode "NewEnumerator1")
      (else
        (Variables|Default|SetBossMode "NewEnumerator2")))))

(fn GotoNextLevel
  (bind _array_element (Utilities|Array|ForEachLoopwithBreak (Variables|/Game/Blueprints/Comunes/GI_Game.GI_Game_C|GetLevelData (CallFunction|GetGIReference)) :!label _label)
    (:LoopBody
      (bind _returnvalue (Game|GetCurrentLevelName true))
      (if (Utilities|Enum|Equal(Enum) _returnvalue (Utilities|String|ToString(Name) (.level_name _array_element)))
        (LocalVariables|SetnextLevel (.level_name _array_element))
        (goto _label Break)))
    (:Completed
      (Game|OpenLevel(byName) (.next_level _array_element)))))