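; BP_Cell is a room grid cell that shows its coordinate and can hold one item.
; On BeginPlay it writes its X,Y Coordinate to a text render and applies its Material to the cube.
; SetContent returns false if Item is already valid; otherwise it stores the item, attaches it snapped to the Scene component with world rotation and scale kept, and returns true.
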(event `self.ReceiveBeginPlay`
  (bind (_coordinate_x _coordinate_y) (break `/Game/Structs/S_CoordenateFloor` (`self.Coordinate`)))
  (`TextRenderComponent.K2_SetText` (`self.TextRender`) (`|FormatText` "({X},{Y})" _coordinate_x _coordinate_y))
  (`PrimitiveComponent.SetMaterial` (`self.Cube`) 0 (`self.Material`)))

(fn `setContent`
  (params (Item :type "/Game/Blueprints/Rooms/BP_Item Object Reference"))
  (returns (CantAdded :type Boolean))
  (`self.Item`
    (:`then`
      (return false))
    (:`else`
      (bind _output_get (set `self.Item` Item))
      (`self.K2_AttachToComponent` _output_get (`self.Scene`) "None" "SnapToTarget" "KeepWorld" "KeepWorld" true)
      (return true))))

(fn `UserConstructionScript`)