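; BP_Board procedurally builds a room as a grid of BP_Cell actors and scatters decorative items across it on BeginPlay.
; Width, height and item count scale with the GameInstance difficulty multiplier.
; Border cells become taller gravel blocks, inner cells get a wood floor, and each is stored in a coordinate-keyed map.
; Randomly chosen BP_Items target non-border cells and are destroyed if the cell rejects them.
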(event `self.ReceiveBeginPlay`
  (`self.AddFloor`)
  (for _ (range (+ (* (`self.ItemsToSpawn`) (`/Game/Blueprints/Comunes/GI_Game.MultiplierDifficulty` (`/Game/Blueprints/FunctionsLibrary/BFL_General.getGIReference`))) 1))
    ;[1 1 1] Nos interesa que no se pongan en los bordes
    (`self.spawnItemDecorator` (make `/Game/Structs/S_CoordenateFloor` (`KismetMathLibrary.RandomIntegerInRange` 1 (- (`self.Width`) 1)) (`KismetMathLibrary.RandomIntegerInRange` 1 (- (`self.Height`) 1))))))

(fn `AddFloor`
  (bind _multiplierdifficulty (`/Game/Blueprints/Comunes/GI_Game.MultiplierDifficulty` (`/Game/Blueprints/FunctionsLibrary/BFL_General.getGIReference`)))
  (bind _output_get (set `self.Width` (* (`self.Width`) _multiplierdifficulty)))
  (bind _output_get_2 (set `self.Height` (* _multiplierdifficulty (`self.Height`))))
  (`self.CreateFloor` _output_get _output_get_2))

(fn `CreateFloor`
  (params (Width :type Integer) (Height :type Integer))
  (locals (X :type Integer) (Y :type Integer))
  (bind (_scalez _material) (`self.setScale` (`local.X`) (`local.Y`)))
  (bind _s_coordenatefloor (make `/Game/Structs/S_CoordenateFloor` (`local.X`) (`local.Y`)))
  (for _index (range (+ Width 1))
    (set `local.X` _index)
    (for _index_2 (range (+ Height 1))
      (set `local.Y` _index_2)
      (bind _returnvalue (`|SpawnActorFromClass` "/Game/Blueprints/Rooms/BP_Cell.BP_Cell_C" (`KismetMathLibrary.MakeTransform` (`KismetMathLibrary.MakeVector` (`KismetMathLibrary.Conv_IntToDouble` (* (`local.Y`) 100)) (`KismetMathLibrary.Conv_IntToDouble` (* (`local.X`) 100))) (struct) (`KismetMathLibrary.MakeVector` 1.0 1.0 _scalez)) "Undefined" "OverrideRootScale" null _s_coordenatefloor _material null))
      (`BlueprintMapLibrary.Map_Add` (`self.Board`) _s_coordenatefloor _returnvalue))))

(fn `setScale`
  (params (X :type Integer) (Y :type Integer))
  (returns (scaleZ :type "Float (double-precision)") (Material :type "Material Object Reference"))
  (bind _returnvalue (or (or (== X 0) (== X (`self.Width`))) (or (== Y 0) (== Y (`self.Height`)))))
  (return (select `bool` _returnvalue :`false` 1.0 :`true` 5.0) (select `bool` _returnvalue :`false` "/Game/StarterContent/Materials/M_Wood_Floor_Walnut_Worn.M_Wood_Floor_Walnut_Worn" :`true` "/Game/StarterContent/Materials/M_Ground_Gravel.M_Ground_Gravel" :!type "Material Object Reference")))

(fn `spawnItemDecorator`
  (params (Coordenate :type "/Game/Structs/S_CoordenateFloor Structure"))
  (locals (ItemsArray :type "Array of PaperSprite Object Reference"))
  (bind _returnvalue (`|SpawnActorFromClass` "/Game/Blueprints/Rooms/BP_Item.BP_Item_C" (`KismetMathLibrary.MakeTransform` (0.0 0.0 0.0)) "AlwaysSpawn" "OverrideRootScale" null (`KismetArrayLibrary.Array_Random` (`local.ItemsArray`)) Coordenate null))
  (bind _cantadded (`/Game/Blueprints/Rooms/BP_Cell.setContent` (`BlueprintMapLibrary.Map_Find` (`self.Board`) Coordenate) _returnvalue))
  (if (not _cantadded)
    (`self.K2_DestroyActor` _returnvalue)))

(fn `UserConstructionScript`)