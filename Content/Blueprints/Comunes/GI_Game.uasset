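; GI_Game, apparently the Game Instance, exposes access to the player-progress save game.
; The progress getter calls LoadGame when the cached save object is invalid, then returns that variable.
; SaveGame and LoadGame are stubs that only print Spanish status messages, so neither touches disk or sets the object.
; DeleteSaveData deletes the progress slot for user index 0.
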(fn `deleteSaveData`
  (`GameplayStatics.DeleteGameInSlot` (`self.getPlayerProgressSlotName`)))

(fn `getPlayerProgressSG`
  (returns (SG_PlayerProgress :type "/Game/Blueprints/SaveGame/SG_PlayerProgress Object Reference"))
  (`self.SG_PlayerProgress`
    (:`then`
      _)
    (:`else`
      (`self.loadGame`)))
  (return (`self.SG_PlayerProgress`)))

(fn `getPlayerProgressSlotName`
  (returns (SlotPlayerProgress1 :type String))
  (locals (SlotPlayerProgress :type String :default "SlotPlayerProgress"))
  (return (`local.SlotPlayerProgress`)))

(fn `loadGame`
  (`KismetSystemLibrary.PrintString` "Partida Cargada")
  (return))

(fn `saveGame`
  (`KismetSystemLibrary.PrintString` "Partida Guardada")
  (return))