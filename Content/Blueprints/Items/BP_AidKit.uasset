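; Aid kit pickup that heals a Hero2D when it overlaps the kit's Box component.
; The heal amount comes from a math expression on the hero's HealthMax, read from its BPCHealth component.
; Healing is sent through ApplyDamage as negative damage, relying on the hero's damage handling to restore health.
; The kit then prints a debug string and destroys itself, making it single-use.
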(event OnComponentBeginOverlap(Box)
  (params (OverlappedComponent :type Primitive%20Component%20Object%20Reference) (OtherActor :type Actor%20Object%20Reference) (OtherComp :type Primitive%20Component%20Object%20Reference) (OtherBodyIndex :type Integer) (bFromSweep :type Boolean) (SweepResult :type Hit%20Result%20Structure%20%28by%20ref%29))
  (bind _ashero_2d (Utilities|Casting|CastToHero2D OtherActor))
  (Game|Damage|ApplyDamage OtherActor (* (|(HealthMax*({E45D6F91-4B09-0E3A-755F-18B7179E68DC}/100)) (Variables|/Game/Componentes/BPC_Health.BPC_Health_C|GetHealthMax (Variables|/Game/Blueprints/Player/Hero2D.Hero2D_C|GetBPC_Health _ashero_2d))) -1.0) 0 0)
  (Development|PrintString "AidKit")
  (Actor|DestroyActor))

(fn ConstructionScript)