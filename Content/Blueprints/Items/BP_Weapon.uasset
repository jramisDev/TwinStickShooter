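; BP_Weapon is a weapon pickup item that grants its configured weapon to the Hero2D player.
; The construction script sets the paper sprite to match the selected weapon type (pistol, Vulcan or missiles).
; When a Hero2D overlaps its box, it finds the matching entry in its WeaponData array, passes it to AddWeapon, then destroys itself.
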(event `self.Box.OnComponentBeginOverlap`
  (params (OverlappedComponent :type "PrimitiveComponent Object Reference") (OtherActor :type "Actor Object Reference") (OtherComp :type "PrimitiveComponent Object Reference") (OtherBodyIndex :type Integer) (bFromSweep :type Boolean) (SweepResult :type "HitResult Structure (by ref)"))
  (bind _ashero_2d (cast `/Game/Blueprints/Player/Hero2D` OtherActor))
  (for _array_element (`self.WeaponData`)
    (if (`|EnumEquality` (`.WEAPON_42_86BE3C51473B5F3F5A2E2D9A44A78369` (break `/Game/Structs/S_Weapon` _array_element)) (`self.Weapon`))
      (`/Game/Blueprints/Player/Hero2D.addWeapon` _ashero_2d _array_element)
      (break)))
  (`self.K2_DestroyActor`))

(fn `displayWeapon`
  (`PaperSpriteComponent.SetSprite` (`self.PaperSprite`) (select `/Game/Blueprints/Enums/E_Weapons` (`self.Weapon`) :`NewEnumerator0` "/Game/Assets/IconsPixels/pistol_Sprite.pistol_Sprite" :`NewEnumerator1` "/Game/Assets/IconsPixels/pistol1_Sprite.pistol1_Sprite" :`NewEnumerator2` "/Game/Assets/IconsPixels/pistol2_Sprite.pistol2_Sprite" :!type "PaperSprite Object Reference")))

(fn `UserConstructionScript`
  (`self.displayWeapon`))